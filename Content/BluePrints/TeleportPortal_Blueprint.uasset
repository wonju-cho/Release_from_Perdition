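; Teleport portal that unlocks through key pickups and sends the shadow runner character to a specific checkpoint.
; Its particle effect starts hidden while Tick polls the count of remaining key actors against its Index value.
; On a match it triggers once, revealing the effect and dropping itself vertically into place.
; Character overlap searches all checkpoints for a hard-coded index and teleports the player pawn there, without checking the triggered flag.
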(event `self.ReceiveBeginPlay`
  (`SceneComponent.SetVisibility` (`self.ParticleSystemComponent`) false false))

(event `self.ReceiveTick`
  (params (DeltaSeconds :type "Float (single-precision)"))
  (if (not (`self.isTriggered`))
    (bind _outactors (`GameplayStatics.GetAllActorsOfClass` "/Game/BluePrints/KeyPickupActor_BP.KeyPickupActor_BP_C"))
    (if (== (`KismetArrayLibrary.Array_Length` _outactors) (`self.Index`))
      (set `self.isTriggered` true)
      (`SceneComponent.SetVisibility` (`self.ParticleSystemComponent`) true false)
      (`self.K2_TeleportTo` self (- (`self.K2_GetActorLocation` self) (0.0 0.0 1500.0)) (`self.K2_GetActorRotation` self)))))

(event `self.ReceiveActorBeginOverlap`
  (params (OtherActor :type "Actor Object Reference"))
  (if (== (`GameplayStatics.GetObjectClass` OtherActor) "/Game/BluePrints/ShadowRunnerCharacter_BP.ShadowRunnerCharacter_BP_C")
    (bind _outactors (`GameplayStatics.GetAllActorsOfClass` "/Game/BluePrints/CheckPoint_BP.CheckPoint_BP_C"))
    (for _index (range (+ (`KismetArrayLibrary.Array_Length` _outactors) 1))
      (bind _output (`|GetArrayItem` _outactors _index))
      (if (== (`/Game/BluePrints/CheckPoint_BP.Index` _output) 5)
        (`self.K2_TeleportTo` :`self` (`GameplayStatics.GetPlayerPawn` 0) :`DestLocation` (`self.K2_GetActorLocation` _output))))))

(fn `UserConstructionScript`)