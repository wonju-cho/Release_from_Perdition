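; TextSpawnerActor_BP is a trigger actor that shows assistant dialogue text while the ShadowRunner character stands inside it.
; On overlap begin with ShadowRunnerCharacter_BP, it creates an AssistantText widget, adds it to the viewport and fills its dialogue block from the actor's ActorText variable.
; On overlap end with that same class, it removes the widget from the screen.
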(event `self.ReceiveBeginPlay`)

(event `self.ReceiveActorBeginOverlap`
  (params (OtherActor :type "Actor Object Reference"))
  (if (== (`GameplayStatics.GetObjectClass` OtherActor) "/Game/BluePrints/ShadowRunnerCharacter_BP.ShadowRunnerCharacter_BP_C")
    (bind _returnvalue (`|CreateWidget` "/Game/BluePrints/AssistantText.AssistantText_C"))
    (`UserWidget.AddToViewport` _returnvalue 0)
    (`TextBlock.SetText` (`/Game/BluePrints/AssistantText.DialogueTextBlock` _returnvalue) (`self.ActorText`))))

(event `self.ReceiveActorEndOverlap`
  (params (OtherActor :type "Actor Object Reference"))
  (if (== (`GameplayStatics.GetObjectClass` OtherActor) "/Game/BluePrints/ShadowRunnerCharacter_BP.ShadowRunnerCharacter_BP_C")
    (`Widget.RemoveFromParent` (stale `self.ReceiveActorBeginOverlap` _returnvalue))))

(fn `UserConstructionScript`)