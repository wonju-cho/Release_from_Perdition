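; Shadow clone character that shows a tether beam linking it to the player while it exists.
; On BeginPlay it attaches a looked-after beam sound to its capsule and plays the summon montage on the ShadowRunner player's mesh.
; Tick feeds the player's position, converted to the clone's local space, into the ShadowTetherBeam PlayerPos variable.
; The beam sound stops when the clone is destroyed.
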(event `self.ReceiveBeginPlay`
  ;[1 1 1] PlayBeamSFX
  (bind _returnvalue (`GameplayStatics.SpawnSoundAttached` "/Game/Assets/Music/BeamSFX.BeamSFX" (`self.CapsuleComponent`) "None" (0.0 0.0 0.0) (struct) "KeepRelativeOffset" false 1.0 1.0 0.0 null null))
  (set `self.BeamSFX` _returnvalue)
  (bind _asshadow_runner_character_bp (cast `/Game/BluePrints/ShadowRunnerCharacter_BP` (`GameplayStatics.GetPlayerCharacter` 0)))
  (`|PlayMontage` (`/Game/BluePrints/ShadowRunnerCharacter_BP.GetPlayerMesh` _asshadow_runner_character_bp) "/Game/FirstPerson/Animations/Summon_Anim_Montage.Summon_Anim_Montage"))

(event `self.ReceiveDestroyed`
  ;[1 1 1] PlayBeamSFX
  (`AudioComponent.Stop` (`self.BeamSFX`)))

(event `self.ReceiveTick`
  (params (DeltaSeconds :type "Float (single-precision)"))
  (bind _returnvalue (`GameplayStatics.GetPlayerCharacter` 0))
  ;[1 1 1] PlaysBeamEffect
  (`/Engine/EditorBlueprintResources/StandardMacros.IsValid` _returnvalue
    (:`Is Valid`
      (`NiagaraComponent.SetVariableVec3` (`self.ShadowTetherBeam`) "PlayerPos" (`KismetMathLibrary.InverseTransformLocation` (`self.GetTransform`) (`self.K2_GetActorLocation` _returnvalue))))))

(fn `UserConstructionScript`)