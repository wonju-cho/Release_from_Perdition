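; A progression wall that blocks the way while the game state reports living enemies and opens once the count reaches zero.
; Tick polls EnemyCount, using two alternating Gates so each switch between solid and passable fires only once.
; Each switch toggles the mesh's collision and plays or reverses the BarrierFade timeline, scaled by FadeTime, which is meant to drive the dynamic material's opacity.
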(event `self.ReceiveBeginPlay`
  (bind _staticmeshcomponent (`self.StaticMeshComponent`))
  (bind _asnew_game_state (cast `/Game/BluePrints/New_GameState` (`GameplayStatics.GetGameState`)))
  (set `self.GameState` _asnew_game_state)
  (bind _returnvalue (`PrimitiveComponent.CreateDynamicMaterialInstance` _staticmeshcomponent 0 (`PrimitiveComponent.GetMaterial` _staticmeshcomponent 0) "None"))
  (set `self.DynamicMat` _returnvalue)
  (`TimelineComponent.SetPlayRate` (`self.BarrierFade`) (/ 1.0 (`self.FadeTime`))))

(event `self.ReceiveTick`
  (params (DeltaSeconds :type "Float (single-precision)"))
  (bind _barrierfade (`self.BarrierFade`))
  (if (> (`/Game/BluePrints/New_GameState.Enemy_Count` (`self.GameState`)) 0)
    (`/Engine/EditorBlueprintResources/StandardMacros.Gate` false :!label _label
      (:`Exit`
        (`PrimitiveComponent.SetCollisionEnabled` (`self.StaticMeshComponent`) "QueryAndPhysics")
        (`TimelineComponent.PlayFromStart` _barrierfade)
        (`|ExecutionSequence`
          (:`then_0`
            (goto _label :!via `Close`))
          (:`then_1`
            (goto _label_2 :!via `Open`)))))
    (else
      (`/Engine/EditorBlueprintResources/StandardMacros.Gate` false :!label _label_2
        (:`Exit`
          (`PrimitiveComponent.SetCollisionEnabled` (`self.StaticMeshComponent`) "NoCollision")
          (`TimelineComponent.ReverseFromEnd` _barrierfade)
          (`|ExecutionSequence`
            (:`then_0`
              (goto _label_2 :!via `Close`))
            (:`then_1`
              (goto _label :!via `Open`))))))))

(fn `UserConstructionScript`)