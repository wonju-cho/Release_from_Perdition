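; Game state Blueprint that drives adaptive music based on an enemy count.
; Update_Enemy_Count adds a delta to the running count and sets the music target to one while any enemies are counted, otherwise zero.
; Each Tick eases the music state toward that target with a fixed-alpha Lerp, feeds it to the MusicCue's "State" parameter, and applies the scaled volume from ShadowRunnerGameInstance_BP.
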(event `self.ReceiveTick`
  (params (DeltaSeconds :type "Float (single-precision)"))
  (bind _asshadow_runner_game_instance_bp (cast `/Game/BluePrints/ShadowRunnerGameInstance_BP` (`GameplayStatics.GetGameInstance`)))
  (bind _newvolume (`/Game/BluePrints/ShadowRunnerGameInstance_BP.GetVolume` _asshadow_runner_game_instance_bp))
  (`AudioComponent.SetVolumeMultiplier` (`self.Music_Cue`) (* _newvolume 1.2))
  (bind _output_get (set `self.Music State` (`KismetMathLibrary.FClamp` (`KismetMathLibrary.Lerp` (`self.Music State`) (`self.Music State Target`) 0.02))))
  (`AudioComponent.SetFloatParameter` (`self.Music_Cue`) "State" _output_get))

(event `Update_Enemy_Count`
  (params (enemy_counter :type Integer))
  (bind _output_get (set `self.Enemy_Count` (+ (`self.Enemy_Count`) enemy_counter)))
  (if (> _output_get 0)
    (set `self.Music State Target` 1.0)
    (else
      (set `self.Music State Target` 0.0))))

(fn `UserConstructionScript`)