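; First-person player character for ShadowRunner, handling weapon swaps, pause and cheat menus, and death and respawn.
; BeginPlay adds the death widget and equips the rifle, while SwitchWeaponMesh swaps rifle and pistol meshes using offset nudges.
; Tick polls volume from the game instance and watches health, firing a one-shot death sequence with camera shake, low-health widget, input lock and timeline-driven mesh pitch.
; OnRespawn restores input and mesh, then re-arms that sequence.
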(event `Key|F3`
  (params (Key :type "Key Structure"))
  ;[1 1 1] Show FPS
  (:`Pressed`
    (`KismetSystemLibrary.ExecuteConsoleCommand` "stat fps" null)))

(event `self.ReceiveBeginPlay`
  (bind _fp_gun (`self.FP_Gun`))
  ;[1 1 1] Initialize
  (bind _asshadow_runner_game_instance_bp (cast `/Game/BluePrints/ShadowRunnerGameInstance_BP` (`GameplayStatics.GetGameInstance`)))
  (bind _newvolume (`/Game/BluePrints/ShadowRunnerGameInstance_BP.GetVolume` _asshadow_runner_game_instance_bp))
  (bind _output_get (set `self.soundControl` _newvolume))
  (set `self.chaSound` _output_get)
  (bind _returnvalue (`|CreateWidget` "/Game/BluePrints/PlayerDeathWidgetBP.PlayerDeathWidgetBP_C"))
  (`UserWidget.AddToViewport` _returnvalue 0)
  (`SkinnedMeshComponent.SetSkinnedAssetAndUpdate` _fp_gun "/Game/Scifi_Arsenal_Vol2/Skeletal_Meshes/Sci-fi_Rifle_02/SK_Sci-fi_Rifle_02_NoScope_NoMagazine.SK_Sci-fi_Rifle_02_NoScope_NoMagazine" true)
  (`SceneComponent.K2_AddLocalOffset` _fp_gun (0.0 30.0 0.0) false false)
  (set `self.ProjectileClass` "/Game/BluePrints/ShadowRunnerProjectile_BP.ShadowRunnerProjectile_BP_C"))

(event `Key|Escape`
  (params (Key :type "Key Structure"))
  (bind _returnvalue (`GameplayStatics.GetPlayerController` 0))
  (bind _pausemenuref (`self.PauseMenuRef`))
  ;[1 1 1] PauseMenu
  (:`Pressed`
    (`/Engine/EditorBlueprintResources/StandardMacros.IsValid` (`self.PauseMenuRef`)
      (:`Is Valid`
        _)
      (:`Is Not Valid`
        (bind _returnvalue_2 (`|CreateWidget` "/Game/BluePrints/PauseMenu.PauseMenu_C"))
        (set `self.PauseMenuRef` _returnvalue_2)))
    (`GameplayStatics.PlaySound2D` "/Engine/VREditor/Sounds/UI/Floating_UI_Open.Floating_UI_Open" (`self.chaSound`) 1.0 0.0 null null)
    (set `PlayerController.bShowMouseCursor` true _returnvalue)
    (`WidgetBlueprintLibrary.SetInputMode_GameAndUIEx` _returnvalue _pausemenuref "DoNotLock" false)
    (`UserWidget.AddToViewport` _pausemenuref 0)
    (`GameplayStatics.SetGamePaused` true)))

(event `Key|Zero`
  (params (Key :type "Key Structure"))
  (bind _returnvalue (`GameplayStatics.GetPlayerController` 0))
  ;[1 1 1] Cheat Menu
  (:`Pressed`
    (bind _returnvalue_2 (`|CreateWidget` "/Game/BluePrints/CheatWidgetBP.CheatWidgetBP_C"))
    (`GameplayStatics.PlaySound2D` "/Engine/VREditor/Sounds/UI/Floating_UI_Open.Floating_UI_Open" (`self.chaSound`) 1.0 0.0 null null)
    (set `PlayerController.bShowMouseCursor` true _returnvalue)
    (`WidgetBlueprintLibrary.SetInputMode_GameAndUIEx` _returnvalue _returnvalue_2 "DoNotLock" false)
    (`UserWidget.AddToViewport` _returnvalue_2 0)
    (`GameplayStatics.SetGamePaused` true)))

(event `self.SwitchWeaponMesh`
  (params (index :type Integer))
  (bind _fp_gun (`self.FP_Gun`))
  (bind _fp_gun_2 (`self.FP_Gun`))
  ;[1 1 1] Switch Weapon
  (switch `int` index
    (:`0`
      (`SkinnedMeshComponent.SetSkinnedAssetAndUpdate` _fp_gun_2 "/Game/Scifi_Arsenal_Vol2/Skeletal_Meshes/Sci-fi_Rifle_02/SK_Sci-fi_Rifle_02_NoScope_NoMagazine.SK_Sci-fi_Rifle_02_NoScope_NoMagazine" true)
      (`SceneComponent.K2_AddLocalOffset` _fp_gun_2 (0.0 -15.0 -2.5) false false)
      (set `self.ProjectileClass` "/Game/BluePrints/ShadowRunnerProjectile_BP.ShadowRunnerProjectile_BP_C"))
    (:`1`
      (`SkinnedMeshComponent.SetSkinnedAssetAndUpdate` _fp_gun "/Game/Scifi_Arsenal_Vol2/Skeletal_Meshes/Sci-fi_Pistol_02/SK_Sci-fi_Pistol_02_Ironsight_01_Attachment_Laser.SK_Sci-fi_Pistol_02_Ironsight_01_Attachment_Laser" true)
      (`SceneComponent.K2_AddLocalOffset` _fp_gun (0.0 15.0 2.5) false false)
      (set `self.ProjectileClass` "/Game/BluePrints/ShadowRunnerProjectile_BP.ShadowRunnerProjectile_BP_C"))))

(event `self.ReceiveTick`
  (params (DeltaSeconds :type "Float (single-precision)"))
  (bind _returnvalue (`GameplayStatics.GetPlayerController` 0))
  (bind _asshadow_runner_game_instance_bp (cast `/Game/BluePrints/ShadowRunnerGameInstance_BP` (`GameplayStatics.GetGameInstance`)))
  (bind _newvolume (`/Game/BluePrints/ShadowRunnerGameInstance_BP.GetVolume` _asshadow_runner_game_instance_bp))
  (bind _output_get (set `self.soundControl` _newvolume))
  (set `self.chaSound` _output_get)
  (if (<= (`HealthComponent.health` (`self.HealthBar`)) 0.0)
    (`/Engine/EditorBlueprintResources/StandardMacros.DoOnce` false :!label _label
      (:`Completed`
        (`GameplayStatics.PlayWorldCameraShake` "/Game/BluePrints/DeathShake.DeathShake_C" (0.0 0.0 0.0) 0.0 600.0)
        (bind _returnvalue_2 (`|CreateWidget` "/Game/BluePrints/PlayerLowHealthWidget_BP.PlayerLowHealthWidget_BP_C"))
        (`UserWidget.AddToViewport` _returnvalue_2 0)
        (`self.DisableInput` _returnvalue null)
        (`Controller.SetIgnoreLookInput` _returnvalue true)
        (`SceneComponent.SetVisibility` (`self.Mesh`) false true)
        (bind (_direction _newtrack_0) (`Timeline|deathfall` :!via `PlayFromStart`)
          (:`Update`
            (`SceneComponent.K2_SetWorldRotation` (`self.Mesh`) (`KismetMathLibrary.MakeRotator` 0.0 _newtrack_0) false false)))))))

(event `OnRespawn`
  (bind _returnvalue (`GameplayStatics.GetPlayerController` 0))
  (bind _mesh (`self.Mesh`))
  (`self.EnableInput` _returnvalue null)
  (`Controller.ResetIgnoreLookInput` _returnvalue)
  (`SceneComponent.SetVisibility` _mesh true true)
  (`SceneComponent.K2_SetWorldRotation` :`self` _mesh)
  (goto _label :!via `Reset`))

(fn `GetPlayerMesh`
  (returns (`Mesh 1P` :type "SkeletalMeshComponent Object Reference"))
  (return (`self.Mesh1P`)))

(fn `UserConstructionScript`)