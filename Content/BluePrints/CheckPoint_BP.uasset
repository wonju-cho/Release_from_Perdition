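; Checkpoint actor for Shadow Runner that announces itself with on-screen text and a sound when the player character overlaps it.
; On BeginPlay it caches the volume from the game instance to scale the 2D sound effect.
; An IsTriggered flag blocks repeat triggers for a two-second delay, then re-arms.
; The graph stores no respawn or save data.
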(event `self.ReceiveBeginPlay`
  (bind _asshadow_runner_game_instance_bp (cast `/Game/BluePrints/ShadowRunnerGameInstance_BP` (`GameplayStatics.GetGameInstance`)))
  (bind _newvolume (`/Game/BluePrints/ShadowRunnerGameInstance_BP.GetVolume` _asshadow_runner_game_instance_bp)))

(event `self.ReceiveActorBeginOverlap`
  (params (OtherActor :type "Actor Object Reference"))
  (if (`self.isTriggered`)
    _
    (elif (== (`GameplayStatics.GetObjectClass` OtherActor) "/Game/BluePrints/ShadowRunnerCharacter_BP.ShadowRunnerCharacter_BP_C")
      (bind _returnvalue (`|CreateWidget` "/Game/BluePrints/CheckPointText_BP.CheckPointText_BP_C"))
      (`UserWidget.AddToViewport` _returnvalue 0)
      (set `self.isTriggered` true)
      (`GameplayStatics.PlaySound2D` "/Game/Assets/Music/checkpoint_SFX.checkpoint_SFX" (* (stale `self.ReceiveBeginPlay` _newvolume) 0.7) 1.0 0.0 null null)
      (`KismetSystemLibrary.Delay` 2.0)
      (set `self.isTriggered` false))))

(fn `UserConstructionScript`)