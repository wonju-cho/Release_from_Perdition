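; BP_FireParams is a fire effect Blueprint that exposes the colors of a Niagara particle system as variables.
; Its Construction Script pushes smoke, fire, and start and end ember colors into the matching Niagara color parameters, so each placed instance can be tinted in the editor.
; The event graph holds only disabled stub events, so it adds no runtime logic.
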(fn `UserConstructionScript`
  (`FXSystemComponent.SetColorParameter` (`self.Niagara`) "SmokeColor" (`self.SmokeColor`))
  (`FXSystemComponent.SetColorParameter` (`self.Niagara`) "FireColor" (`self.Fire Color`))
  (`FXSystemComponent.SetColorParameter` (`self.Niagara`) "StartEmberColor" (`self.Start Ember Color`))
  (`FXSystemComponent.SetColorParameter` (`self.Niagara`) "EndEmberColor" (`self.End Ember Color`)))